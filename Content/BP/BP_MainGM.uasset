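; Game mode for a two-player host/guest tile duel of up to nine rounds, ending early at five wins.
; A dice roll picks the first player, rerolling on ties.
; Players alternately select tiles, which are compared; round winners lead next, while draws return the lead to that round's first player.
; BP_MainGS holds round, turn and score state, while BP_MainPC receives turn, message and result calls, addressed by controller index.
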(event Custom|OnSelectedDiceNum
  (params (Dice :type BP%20Dice%20Object%20Reference) (SelectedNum :type Integer))
  (bind _maings (Variables|Default|GetMainGS))
  ;[1 1 1] OnSelectDiceNum
  (for _array_element (Variables|Default|GetPlayerCharacters)
    (if (== (Variables|/Game/BP/BP_Character.BP_Character_C|GetMyDice _array_element) Dice)
      (if (== (Game|GetPlayerCharacter 0) _array_element)
        (Variables|/Game/BP/BP_MainGS.BP_MainGS_C|SetHostDiceNum _maings SelectedNum)
        (else
          (Variables|/Game/BP/BP_MainGS.BP_MainGS_C|SetGuestDiceNum _maings SelectedNum)))
      (CallFunction|OnDiceCheck))))

(event Custom|OnDiceRoundStart
  (bind _outactors (Actor|GetAllActorsOfClass "/Game/BP/BP_Character.BP_Character_C"))
  (Variables|Default|SetPlayerCharacters _outactors)
  (if (and (== (Utilities|Array|Length _outactors) 2) (== (Variables|/Game/BP/BP_MainGS.BP_MainGS_C|GetRound (Variables|Default|GetMainGS)) 0))
    (Default|Init (Variables|Default|GetMainGS))
    (bind _returnvalue (Actor|GetActorOfClass "/Game/BP/BP_DiceSpawner.BP_DiceSpawner_C"))
    (bind _output_get (Variables|Default|SetDiceSpawner _returnvalue))
    (Default|SpawnDice _output_get)
    (for (_array_element _array_index) (Variables|Default|GetPlayerCharacters)
      (Variables|/Game/BP/BP_Character.BP_Character_C|SetMyDice _array_element (Utilities|Array|Get(acopy) (Variables|/Game/BP/BP_DiceSpawner.BP_DiceSpawner_C|GetDiceArray (Variables|Default|GetDiceSpawner)) _array_index)))
    (Utilities|FlowControl|Delay 0.2)
    (for _array_element_2 (Variables|/Game/BP/BP_DiceSpawner.BP_DiceSpawner_C|GetDiceArray (Variables|Default|GetDiceSpawner))
      (Default|Init _array_element_2)
      (CallFunction|ShowServerMessage true "주사위를 클릭해서  
굴려주세요" 5.0)
      (CallFunction|ShowServerMessage false "주사위를 클릭해서  
굴려주세요" 5.0))
    (else
      (Development|PrintString "need two players"))))

(event Custom|OnDiceCheck
  ;[1 1 1] OnDiceNumCompare
  (if (Math|Boolean|ANDBoolean (> (Variables|/Game/BP/BP_MainGS.BP_MainGS_C|GetHostDiceNum (Variables|Default|GetMainGS)) 0) (> (Variables|/Game/BP/BP_MainGS.BP_MainGS_C|GetGuestDiceNum (Variables|Default|GetMainGS)) 0) (== (Variables|/Game/BP/BP_MainGS.BP_MainGS_C|GetRound (Variables|Default|GetMainGS)) 0)) ; Player 두명다 주사위를 굴려야함.
    (if (== (Variables|/Game/BP/BP_MainGS.BP_MainGS_C|GetHostDiceNum (Variables|Default|GetMainGS)) (Variables|/Game/BP/BP_MainGS.BP_MainGS_C|GetGuestDiceNum (Variables|Default|GetMainGS))) ; true: 두 플레이어의 주사위 숫자가 같은경우
      (CallFunction|OnDiceRoundStart) ; 주사위 굴리기부터 재시작
      (else
        (bind _output_get (Variables|/Game/BP/BP_MainGS.BP_MainGS_C|SetCurrentPlayerHost (Variables|Default|GetMainGS) (> (Variables|/Game/BP/BP_MainGS.BP_MainGS_C|GetHostDiceNum (Variables|Default|GetMainGS)) (Variables|/Game/BP/BP_MainGS.BP_MainGS_C|GetGuestDiceNum (Variables|Default|GetMainGS))))) ; 주사위가 큰숫자가 나온 플레이어가(host or client)가 다음 선플레이어로 결정됨
        (if _output_get
          (CallFunction|ShowServerMessage true "선 플레이어 입니다" 0.0)
          (CallFunction|ShowServerMessage false "상대가 선 플레이어 입니다" 0.0)
          (else
            (CallFunction|ShowServerMessage false "선 플레이어 입니다" 0.0)
            (CallFunction|ShowServerMessage true "상대가 선 플레이어 입니다" 0.0)))
        (Default|CallOnEndDiceCompare)))))

(event Custom|OnSelectedTileNum
  (params (SelectedTile :type BP%20Tile%20Object%20Reference) (PC :type BP%20Main%20PC%20Object%20Reference))
  (bind _maings (Variables|Default|GetMainGS))
  (if (Utilities|Enum|Equal(Enum) (Variables|/Game/BP/BP_MainGS.BP_MainGS_C|GetGameStep (Variables|Default|GetMainGS)) "NewEnumerator0") ; ture: 타일 고르는 단계인 경우
    (if (Math|Boolean|Equal(Boolean) (Variables|/Game/BP/BP_MainGS.BP_MainGS_C|GetCurrentPlayerHost (Variables|Default|GetMainGS)) (== PC (Game|GetPlayerController 0))) ; True: 현재 순서인 Player가 타일을 선택한경우
      (bind _currentplayerpc (Utilities|GetCurrentPC))
      (Default|RemoveMyTile _currentplayerpc SelectedTile)
      (Default|CallOnSelectedTile SelectedTile)
      (Utilities|SelectTileProcess SelectedTile ; 선택한 타일숫자 적용, 다음 단계로 진행
        (:Host
          (Variables|/Game/BP/BP_MainGS.BP_MainGS_C|SetCurrentPlayerHost _maings true)
          (CallFunction|OnNextRound))
        (:Guest
          (Variables|/Game/BP/BP_MainGS.BP_MainGS_C|SetCurrentPlayerHost _maings false)
          (CallFunction|OnNextRound))
        (:CompareNum
          (Variables|/Game/BP/BP_MainGS.BP_MainGS_C|SetGameStep (Variables|Default|GetMainGS) "NewEnumerator1")
          (CallFunction|ShowServerMessage false "숫자를 비교합니다" 3.0)
          (CallFunction|ShowServerMessage true "숫자를 비교합니다" 3.0)
          (Utilities|FlowControl|Delay 3.0)
          (CallFunction|RoundProcess)
          (CallFunction|DestroyTile)
          (Utilities|ScoreCheck
            (:Next
              (Utilities|NextRound
                (:Next
                  (Utilities|FlowControl|Delay 1.5)
                  (CallFunction|OnNextRound))
                (:End
                  (CallFunction|EndGame :!label _label))))
            (:End
              (goto _label))))))))

(event Custom|OnNextRound
  (Variables|/Game/BP/BP_MainGS.BP_MainGS_C|SetGameStep (Variables|Default|GetMainGS) "NewEnumerator0")
  (bind _currentplayerpc (Utilities|GetCurrentPC))
  (Default|SCSetMyTurn _currentplayerpc true (Variables|/Game/BP/BP_MainGS.BP_MainGS_C|GetCountDown (Variables|Default|GetMainGS)))
  (bind _nextplayerpc (Utilities|GetNextPC))
  (Default|SCSetMyTurn _nextplayerpc false))

(event Custom|RestartGame
  ;[1 1 1] 다시하기
  (Default|Init (Variables|Default|GetMainGS))
  (CallFunction|PlayersInit)
  (CallFunction|OnDiceRoundStart)
  (Default|CallOnRestarted))

(event Custom|OnGameStart
  (Variables|/Game/BP/BP_MainGS.BP_MainGS_C|SetRound (Variables|Default|GetMainGS) 1)
  (CallFunction|OnNextRound))

(event Custom|PlayersInit
  (bind _outactors (Actor|GetAllActorsOfClass "/Script/Engine.PlayerStart"))
  (bind _outactors_2 (Actor|GetAllActorsOfClass "/Game/BP/BP_Character.BP_Character_C"))
  (for (_array_element _array_index) _outactors_2
    (Transformation|SetActorLocation _array_element (Transformation|GetActorLocation (Utilities|Array|Get(acopy) _outactors _array_index)) false false)
    (bind _outactors_3 (Actor|GetAllActorsOfClass "/Game/BP/BP_MainPC.BP_MainPC_C"))
    (for _array_element_2 _outactors_3
      (Default|Init _array_element_2))))

(event EventBeginPlay
  (bind _asbp_main_gs (Utilities|Casting|CastToBP_MainGS (Game|GetGameState)))
  (Variables|Default|SetMainGS _asbp_main_gs))

(event EventTick
  (params (DeltaSeconds :type Float%20%28single-precision%29)))

(event EventOnLogout
  (params (ExitingController :type Controller%20Object%20Reference)))

(fn ConstructionScript)

(fn RoundProcess
  (bind _maings (Variables|Default|GetMainGS))
  (bind _maings_2 (Variables|Default|GetMainGS))
  (bind _maings_3 (Variables|Default|GetMainGS))
  (bind _maings_4 (Variables|Default|GetMainGS))
  (bind _hosttile (Variables|/Game/BP/BP_MainGS.BP_MainGS_C|GetHostTile _maings_4))
  (bind _guesttile (Variables|/Game/BP/BP_MainGS.BP_MainGS_C|GetGuestTile _maings_4))
  (bind _num (Variables|/Game/BP/BP_Tile.BP_Tile_C|GetNum _hosttile))
  (bind _num_2 (Variables|/Game/BP/BP_Tile.BP_Tile_C|GetNum _guesttile))
  (Utilities|>=< (Variables|/Game/BP/BP_Tile.BP_Tile_C|GetNum (Variables|/Game/BP/BP_MainGS.BP_MainGS_C|GetHostTile _maings)) (Variables|/Game/BP/BP_Tile.BP_Tile_C|GetNum (Variables|/Game/BP/BP_MainGS.BP_MainGS_C|GetGuestTile _maings)) ; >: 호스트가 이긴경우\n<: 게스트가 이긴경우
    (:>
      (LocalVariables|SetWinner "NewEnumerator0")
      (Variables|/Game/BP/BP_MainGS.BP_MainGS_C|SetCurrentPlayerHost _maings_2 true)
      (Default|AddRoundResult (Variables|Default|GetMainGS) (LocalVariables|GetWinner) _num _num_2 :!label _label)
      (CallFunction|ShowServerMessage (Utilities|Enum|Equal(Enum) (LocalVariables|GetWinner) "NewEnumerator0") "라운드를 이겼습니다" 3.0)
      (CallFunction|ShowServerMessage (not (Utilities|Enum|Equal(Enum) (LocalVariables|GetWinner) "NewEnumerator0")) "라운드를 졌습니다" 3.0))
    (:==
      (LocalVariables|SetWinner "NewEnumerator1")
      (Variables|/Game/BP/BP_MainGS.BP_MainGS_C|SetCurrentPlayerHost _maings_3 (not (Variables|/Game/BP/BP_MainGS.BP_MainGS_C|GetCurrentPlayerHost _maings_3))) ; 무승부시 이전라운드 선플레이어가 다시 선.
      (Default|AddRoundResult (Variables|Default|GetMainGS) "NewEnumerator1" _num _num_2)
      (CallFunction|ShowServerMessage false "라운드를 비겼습니다" 3.0)
      (CallFunction|ShowServerMessage true "라운드를 비겼습니다" 3.0))
    (:<
      (LocalVariables|SetWinner "NewEnumerator2")
      (Variables|/Game/BP/BP_MainGS.BP_MainGS_C|SetCurrentPlayerHost _maings_2 false)
      (goto _label))))

(fn EndGame
  (bind _outactors (Actor|GetAllActorsOfClass "/Game/BP/BP_MainPC.BP_MainPC_C"))
  (for _array_element _outactors
    (Default|SCPrintResult _array_element)))

(fn DestroyTile
  (Utilities|IsValid (Variables|/Game/BP/BP_MainGS.BP_MainGS_C|GetHostTile (Variables|Default|GetMainGS))
    (:Is%20Valid
      (Actor|DestroyActor (Variables|/Game/BP/BP_MainGS.BP_MainGS_C|GetHostTile (Variables|Default|GetMainGS)))
      (Variables|/Game/BP/BP_MainGS.BP_MainGS_C|SetHostTile (Variables|Default|GetMainGS) 0)
      (Utilities|IsValid (Variables|/Game/BP/BP_MainGS.BP_MainGS_C|GetGuestTile (Variables|Default|GetMainGS))
        (:Is%20Valid
          (Actor|DestroyActor (Variables|/Game/BP/BP_MainGS.BP_MainGS_C|GetGuestTile (Variables|Default|GetMainGS)))
          (Variables|/Game/BP/BP_MainGS.BP_MainGS_C|SetGuestTile (Variables|Default|GetMainGS) 0))))))

(fn ShowServerMessage
  (params (bHost :type Boolean) (Message :type String) (MilliSec :type Float%20%28single-precision%29))
  (bind _asplayer_controller (Utilities|Casting|CastToPlayerController (Utilities|SelectObject (Game|GetPlayerController 0) (Game|GetPlayerController 1) bHost)))
  (Utilities|SendServerMessage _asplayer_controller Message MilliSec))