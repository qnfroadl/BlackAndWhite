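; Player controller for a two-player, turn-based tile-picking game, linking the local HUD, pawn and game mode.
; SC_ events drive HUD messages, score visibility and turns, starting a countdown that triggers the pawn's random pick on timeout.
; Tile selection clears the countdown and passes through CS_SelectedTile to the game mode.
; A looping timer replays GameState round results one by one, using authority to choose host or guest perspective.
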(event Custom|SC_ShowServerMessage
  (params (Message :type String) (MilliSec :type Float%20%28single-precision%29))
  (Default|SetServerMessage (Variables|Default|GetMainHUD) Message MilliSec))

(event Custom|SC_SetVisibleScore
  (params (visible :type Boolean))
  (Default|SetVisibleScore (Variables|Default|GetMainHUD) visible))

(event Custom|SC_SetMyTurn
  (params (MyTurn :type Boolean) (Count :type Integer))
  (if MyTurn
    (Default|SetServerMessage (Variables|Default|GetMainHUD) "타일을 선택해주세요" 0.0)
    (CallFunction|SetCountDownTimer Count)
    (else
      (Default|SetVisibleCount (Variables|Default|GetMainHUD) false)
      (Default|SetServerMessage (Variables|Default|GetMainHUD) "상대를 기다리는중" 0.0))))

(event Custom|CS_SelectedTile
  (params (SelectedTile :type BP%20Tile%20Object%20Reference))
  (bind _asbp_main_gm (Utilities|Casting|CastToBP_MainGM (Game|GetGameMode)))
  (Default|OnSelectedTileNum _asbp_main_gm SelectedTile self))

(event Custom|TimeCheck
  (bind _output_get (Variables|Default|SetCountDown (- (Variables|Default|GetCountDown) 1)))
  (if (< _output_get 1) ; 랜덤으로 강제 선택
    (bind _asbp_character (Utilities|Casting|CastToBP_Character (Pawn|GetControlledPawn)))
    (Default|OnTimeOutRandomTile _asbp_character)))

(event Custom|SelectedTile
  (params (SelectedTile :type BP%20Tile%20Object%20Reference))
  (if (Utilities|Time|IsValidTimerHandle (Variables|Default|GetCountTimer))
    (Utilities|Time|ClearandInvalidateTimerbyHandle (Variables|Default|GetCountTimer))
    (Variables|Default|SetCountTimer "")
    (Default|SetVisibleCount (Variables|Default|GetMainHUD) false))
  (CallFunction|CSSelectedTile SelectedTile))

(event Custom|SetCountDownTimer
  (params (Count :type Integer))
  (if (> Count 0)
    (Variables|Default|SetCountDown Count)
    (bind _returnvalue (Utilities|Time|SetTimerbyEvent (delegate Custom|TimeCheck) 1.0 true))
    (Variables|Default|SetCountTimer _returnvalue)
    (Default|SetVisibleCount (Variables|Default|GetMainHUD) true)
    (else
      (Default|SetVisibleCount (Variables|Default|GetMainHUD) false))))

(event Custom|TimeoutPrintResult
  (bind _mainhud (Variables|Default|GetMainHUD))
  (Networking|SwitchHasAuthority
    (:Authority
      (Default|PrintRoundResult _mainhud (Utilities|Enum|Equal(Enum) (.winner (Utilities|Array|Get(acopy) (Variables|/Game/BP/BP_MainGS.BP_MainGS_C|GetRoundResultArray (Variables|Default|GetMain%20GS)) (Variables|Default|GetResultIndex))) "NewEnumerator0") (.hostnum (Utilities|Array|Get(acopy) (Variables|/Game/BP/BP_MainGS.BP_MainGS_C|GetRoundResultArray (Variables|Default|GetMain%20GS)) (Variables|Default|GetResultIndex))) (.guestnum (Utilities|Array|Get(acopy) (Variables|/Game/BP/BP_MainGS.BP_MainGS_C|GetRoundResultArray (Variables|Default|GetMain%20GS)) (Variables|Default|GetResultIndex))) (Utilities|Enum|Equal(Enum) (.winner (Utilities|Array|Get(acopy) (Variables|/Game/BP/BP_MainGS.BP_MainGS_C|GetRoundResultArray (Variables|Default|GetMain%20GS)) (Variables|Default|GetResultIndex))) "NewEnumerator1")) ; 호스트일때
    )
    (:Remote
      (Default|PrintRoundResult _mainhud (Utilities|Enum|Equal(Enum) (.winner (Utilities|Array|Get(acopy) (Variables|/Game/BP/BP_MainGS.BP_MainGS_C|GetRoundResultArray (Variables|Default|GetMain%20GS)) (Variables|Default|GetResultIndex))) "NewEnumerator2") (.guestnum (Utilities|Array|Get(acopy) (Variables|/Game/BP/BP_MainGS.BP_MainGS_C|GetRoundResultArray (Variables|Default|GetMain%20GS)) (Variables|Default|GetResultIndex))) (.hostnum (Utilities|Array|Get(acopy) (Variables|/Game/BP/BP_MainGS.BP_MainGS_C|GetRoundResultArray (Variables|Default|GetMain%20GS)) (Variables|Default|GetResultIndex))) (Utilities|Enum|Equal(Enum) (.winner (Utilities|Array|Get(acopy) (Variables|/Game/BP/BP_MainGS.BP_MainGS_C|GetRoundResultArray (Variables|Default|GetMain%20GS)) (Variables|Default|GetResultIndex))) "NewEnumerator1")) ; 게스트일때
    ))
  (bind _output_get (Variables|Default|SetResultIndex (+ (Variables|Default|GetResultIndex) 1)))
  (if (>= _output_get (Utilities|Array|Length (Variables|/Game/BP/BP_MainGS.BP_MainGS_C|GetRoundResultArray (Variables|Default|GetMain%20GS))))
    (Utilities|Time|ClearandInvalidateTimerbyHandle (Variables|Default|GetResultTimer))
    (Variables|Default|SetResultTimer "")
    (Variables|Default|SetResultIndex 0)))

(event Custom|RemoveMyTile
  (params (SelectedTile :type BP%20Tile%20Object%20Reference))
  (bind _asbp_character (Utilities|Casting|CastToBP_Character (Pawn|GetControlledPawn)))
  (Utilities|Array|RemoveItem (Variables|/Game/BP/BP_Character.BP_Character_C|GetMyTileArray _asbp_character) SelectedTile))

(event Custom|SC_PrintResult
  (bind _returnvalue (Utilities|Time|SetTimerbyEvent (delegate Custom|TimeoutPrintResult) 1.0 true))
  (Variables|Default|SetResultTimer _returnvalue))

(event EventBeginPlay
  (Input|SetInputModeGameOnly (Game|GetPlayerController 0))
  (if (Pawn|IsLocalPlayerController)
    (bind _asbp_main_hud (Utilities|Casting|CastToBP_MainHUD (HUD|GetHUD)))
    (Variables|Default|SetMainHUD _asbp_main_hud)
    (bind _asbp_main_gs (Utilities|Casting|CastToBP_MainGS (Game|GetGameState)))
    (Variables|Default|SetMain%20GS _asbp_main_gs)))

(event EventTick
  (params (DeltaSeconds :type Float%20%28single-precision%29)))

(fn ConstructionScript)