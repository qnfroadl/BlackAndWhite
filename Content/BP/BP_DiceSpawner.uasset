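; BP_DiceSpawner is an actor that spawns and resets a pair of dice on the server.
; SpawnDice runs only with authority, creating two BP_Dice at the spawner's root transform on first use and storing them in DiceArray.
; Later calls reuse those dice, moving them back to the spawner's location and stacking them vertically by array index.
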(event Custom|SpawnDice
  (bind _defaultsceneroot (Variables|Default|GetDefaultSceneRoot))
  (bind _returnvalue (Transformation|GetWorldLocation _defaultsceneroot))
  (Networking|SwitchHasAuthority
    (:Authority
      (if (== (Utilities|Array|Length (Variables|Default|GetDiceArray)) 0)
        (for _index (range 0 1)
          (bind _returnvalue_2 (Game|SpawnActorfromClass "/Game/BP/BP_Dice.BP_Dice_C" (Transformation|GetWorldTransform (Variables|Default|GetDefaultSceneRoot)) "AdjustIfPossibleButAlwaysSpawn" 0 0))
          (Utilities|Array|Add (Variables|Default|GetDiceArray) _returnvalue_2))
        (else
          (for (_array_element _array_index) (Variables|Default|GetDiceArray)
            (Transformation|SetActorLocation _array_element (Math|Vector|MakeVector (.x _returnvalue) (.y _returnvalue) (+ (.z _returnvalue) (Math|Conversions|ToFloat(Integer) (* _array_index 100)))) false false)))))))

(event EventBeginPlay)

(fn ConstructionScript)