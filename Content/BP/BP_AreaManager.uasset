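; BP_AreaManager is an area manager that can reset a set of BP_Tile actors to their starting layout.
; On BeginPlay it records each tile's mesh world transform and Num value in parallel arrays.
; Respawn destroys the current tiles, spawns new ones at the saved locations and rotations, initializes each with its saved Num, and rebuilds TileArray.
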(event Custom|Respawn
  (for _array_element (Variables|Default|GetTileArray)
    (Utilities|IsValid _array_element
      (:Is%20Valid
        (Actor|DestroyActor _array_element))))
  (Utilities|Array|Clear (Variables|Default|GetTileArray))
  (for (_array_element_2 _array_index) (Variables|Default|GetTileArrayLocation)
    (bind _returnvalue (Game|SpawnActorfromClass "/Game/BP/BP_Tile.BP_Tile_C" (Math|Transform|MakeTransform (.location _array_element_2) (.rotation _array_element_2) "1,1,1") "AlwaysSpawn" 0 0))
    (Default|Init _returnvalue (Utilities|Array|Get(acopy) (Variables|Default|GetTileArrayNum) _array_index))
    (Utilities|Array|Add (Variables|Default|GetTileArray) _returnvalue)))

(event EventBeginPlay
  (for _array_element (Variables|Default|GetTileArray)
    (Utilities|Array|Add (Variables|Default|GetTileArrayLocation) (Transformation|GetWorldTransform (Variables|/Script/Engine.StaticMeshActor|GetStaticMeshComponent _array_element)))
    (Utilities|Array|Add (Variables|Default|GetTileArrayNum) (Variables|/Game/BP/BP_Tile.BP_Tile_C|GetNum _array_element))))

(fn ConstructionScript)