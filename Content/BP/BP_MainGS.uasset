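; BP_MainGS is a GameState that tracks a round-based Host versus Guest dice match: step, countdown, round, wins, dice numbers and tiles.
; An Init event resets that state and clears the round history.
; AddRoundResult logs each round's winner flag and both numbers, then increments the matching win counter.
; Several variables, including wins, round, step and current player, have RepNotify functions, all currently empty.
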(event Custom|Init
  (Utilities|Array|Clear (Variables|Default|GetRoundResultArray))
  (Variables|Default|SetGameStep "NewEnumerator3")
  (Variables|Default|SetCountDown 300)
  (Variables|Default|SetRound 1)
  (Variables|Default|SetHostWin 0)
  (Variables|Default|SetGuestWin 0)
  (Variables|Default|SetHostDiceNum 0)
  (Variables|Default|SetGuestDiceNum 0)
  (Variables|Default|SetHostTile 0)
  (Variables|Default|SetGuestTile 0)
  (Development|PrintString "Init GameState"))

(event EventBeginPlay)

(event EventTick
  (params (DeltaSeconds :type Float%20%28single-precision%29)))

(fn ConstructionScript)

(fn AddRoundResult
  (params (bHostWin :type Boolean) (HostNum :type Integer) (GuestNum :type Integer))
  (Utilities|Array|Add (Variables|Default|GetRoundResultArray) (Utilities|Struct|MakeBP_RoundResult bHostWin HostNum GuestNum))
  (if bHostWin
    (Variables|Default|SetHostWin (+ (Variables|Default|GetHostWin) 1))
    (else
      (Variables|Default|SetGuestWin (+ (Variables|Default|GetGuestWin) 1)))))

(fn OnRepHostWin)

(fn OnRepGuestWin)

(fn OnRepRound)

(fn OnRepHostDiceNum)

(fn OnRepGameStep)

(fn OnRepCurrentPlayerHost)