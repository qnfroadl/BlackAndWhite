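; BP_TimeText is a text render actor that displays a seconds countdown, or a fixed Value text when Infinity is set.
; On BeginPlay the authority sets the initial text and, unless Infinity is set, starts a looping one-second timer that decrements Sec.
; OnRep_Sec refreshes the displayed number whenever Sec changes.
; Nothing in the graph stops the timer at zero.
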(event Custom|TimeCheck
  (Variables|Default|SetSec (- (Variables|Default|GetSec) 1)))

(event EventBeginPlay
  (Networking|SwitchHasAuthority
    (:Authority
      (if (Variables|Default|GetbInfinity)
        (Rendering|Components|TextRender|SetText (Variables|Default|GetTextRender) (Variables|Default|GetValue))
        (else
          (Rendering|Components|TextRender|SetText (Variables|Default|GetTextRender) (Utilities|Text|ToText(Integer) (Variables|Default|GetSec)))
          (bind _returnvalue (Utilities|Time|SetTimerbyEvent (delegate Custom|TimeCheck) 1.0 true))
          (Variables|Default|SetSecTimer _returnvalue))))))

(fn ConstructionScript)

(fn OnRepSec
  (Rendering|Components|TextRender|SetText (Variables|Default|GetTextRender) (Utilities|Text|ToText(Integer) (Variables|Default|GetSec))))