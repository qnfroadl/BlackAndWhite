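; BP_Tile is a numbered board tile that lifts when hovered and exposes a selection event.
; The construction script uses Num's parity to set a black or white dynamic material with contrasting number text.
; OnHover drives a timeline that raises the tile from its starting Z, with a retriggerable delay reversing it afterward.
; OnSelect is a stub that only prints and casts the game mode to BP_MainGM.
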(event Custom|OnHover
  (bind _returnvalue (Transformation|GetActorLocation))
  ;[1 1 1] Hover
  (bind _alpha (Timeline|타임라인 Play)
    (:Update
      (Transformation|SetActorLocation (Math|Vector|MakeVector (.x _returnvalue) (.y _returnvalue) (+ (Variables|Default|GetZOrigin) (* _alpha 2e+01))) false false)
      (Utilities|FlowControl|RetriggerableDelay 0.2)
      (Timeline|타임라인 Reverse))))

(event Custom|OnSelect
  (params (PC :type Player%20Controller%20Object%20Reference))
  (Development|PrintString "OnSelect")
  (Utilities|Casting|CastToBP_MainGM (Game|GetGameMode)))

(event EventBeginPlay
  (Variables|Default|SetZOrigin (.z (Transformation|GetActorLocation))))

(event Collision|EventActorBeginOverlap
  (params (OtherActor :type Actor%20Object%20Reference)))

(event EventTick
  (params (DeltaSeconds :type Float%20%28single-precision%29)))

(fn ConstructionScript
  (bind _textrender (Variables|Default|GetTextRender))
  (bind _returnvalue (Rendering|Material|CreateDynamicMaterialInstance "/Game/Materials/MI_Tile.MI_Tile" "" "None" :!class /Script/Engine.KismetMaterialLibrary))
  (Rendering|Material|SetVectorParameterValue _returnvalue "Color" (Math|Color|SelectColor "(R=0.000000,G=0.000000,B=0.000000,A=1.000000)" "(R=1.000000,G=1.000000,B=1.000000,A=1.000000)" (== (Math|Integer|%(Integer) (Variables|Default|GetNum) 2) 0)) :!class /Script/Engine.MaterialInstanceDynamic)
  (Rendering|Material|SetMaterial (Variables|Debug|GetStaticMeshComponent) 0 _returnvalue)
  (Rendering|Components|TextRender|SetText _textrender (Utilities|Text|ToText(Integer) (Variables|Default|GetNum)))
  (Rendering|Components|TextRender|SetTextRenderColor _textrender (Math|Conversions|ToColor(LinearColor) (Math|Color|SelectColor "(R=1.000000,G=1.000000,B=1.000000,A=1.000000)" "(R=0.000000,G=0.000000,B=0.000000,A=1.000000)" (== (Math|Integer|%(Integer) (Variables|Default|GetNum) 2) 0)))))